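; BP_SpaceHud sets up the on-screen UI for the GalaxyShooter game: a flight UI and a custom mouse cursor.
; On BeginPlay it creates the WBP_FlightUI and WBP_Cursor widgets, adds both to the viewport and stores references to them.
; Every Tick it moves the cursor widget to the first player controller's mouse position, with DPI scale removed.
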(event `self.ReceiveBeginPlay`
  (`|ExecutionSequence`
    (:`then_0`
      (bind _returnvalue (`|CreateWidget` "/Game/GalaxyShooter/UI/WBP_FlightUI.WBP_FlightUI_C"))
      (`UserWidget.AddToViewport` _returnvalue 0)
      (set `self.WBP_FlightUI` _returnvalue))
    (:`then_1`
      (bind _returnvalue_2 (`|CreateWidget` "/Game/GalaxyShooter/UI/WBP_Cursor.WBP_Cursor_C"))
      (`UserWidget.AddToViewport` _returnvalue_2 0)
      (set `self.WBP_Cursor` _returnvalue_2))))

(event `self.ReceiveTick`
  (params (DeltaSeconds :type "Float (single-precision)"))
  (bind (_locationx _locationy) (`PlayerController.GetMousePosition` (`GameplayStatics.GetPlayerController` 0)))
  (`UserWidget.SetPositionInViewport` (`self.WBP_Cursor`) (`KismetMathLibrary.MakeVector2D` _locationx _locationy) true))

(fn `UserConstructionScript`)