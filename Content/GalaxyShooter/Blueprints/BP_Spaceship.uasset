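; Player spaceship for GalaxyShooter, steered by cursor offset from screen center with mouse-wheel thrust.
; A sphere trace under the cursor fills a HUD scan timer, then engages autopilot on the hit actor if Interact has armed it.
; Autopilot turns toward and approaches the target, with Boost toggling global time dilation.
; Arrival starts a comet mining minigame or opens the station level, while manual collisions destroy comets.
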(event `self.ReceiveTick`
  (params (DeltaSeconds :type "Float (single-precision)"))
  (bind _capsulecomponent (`self.CapsuleComponent`))
  (bind _capsulecomponent_2 (`self.CapsuleComponent`))
  (bind (_worldlocation _worlddirection) (`PlayerController.DeprojectMousePositionToWorld` (`GameplayStatics.GetPlayerController` 0)))
  (bind (_locationx _locationy) (`PlayerController.GetMousePosition` (`GameplayStatics.GetPlayerController` 0)))
  (bind (_returnvalue_roll _returnvalue_pitch _returnvalue_yaw) (`KismetMathLibrary.BreakRotator` (`SceneComponent.K2_GetComponentRotation` _capsulecomponent_2)))
  (bind (_returnvalue_x _returnvalue_y) (`KismetMathLibrary.BreakVector2D` (* (`self.ScreenDirection`) (0.001 0.001))))
  (bind _returnvalue (* _returnvalue_x -1.0))
  (if (not (`self.MineMiniGame`))
    (`|ExecutionSequence`
      (:`then_0`
        (if (`self.Autopilot`)
          ;[1 1 1] AutopilotFlight
          (switch `/Game/GalaxyShooter/Blueprints/AutopilotState` (`self.AutoPilotState`)
            (:`NewEnumerator2`
              (set `self.Autopilot` false)
              (bind _asbp_space_hud (cast `/Game/GalaxyShooter/Game/BP_SpaceHud` (`PlayerController.GetHUD` (`GameplayStatics.GetPlayerController` 0))))
              (`Widget.SetVisibility` (`/Game/GalaxyShooter/Game/BP_SpaceHud.WBP_Cursor` _asbp_space_hud) "Visible"))
            (:`NewEnumerator1`
              (`SceneComponent.K2_SetWorldRotation` _capsulecomponent (`KismetMathLibrary.RInterpTo` (`SceneComponent.K2_GetComponentRotation` _capsulecomponent) (`KismetMathLibrary.FindLookAtRotation` (`SceneComponent.K2_GetComponentLocation` _capsulecomponent) (`self.K2_GetActorLocation` (`self.AutoPilotDestinationActor`))) DeltaSeconds 1.0) false false)
              (`self.AddMovementInput` (`self.GetActorForwardVector`) 2.0)))
          (else
            ;[1 1 1] FlightControll
            (`|ExecutionSequence`
              (:`then_0`
                (`|ExecutionSequence`
                  (:`then_0`
                    (set `self.ScreenDirection` (- (/ (`WidgetLayoutLibrary.GetViewportSize`) (2.0 2.0)) (`KismetMathLibrary.MakeVector2D` _locationx _locationy))))
                  (:`then_1`
                    (`SceneComponent.K2_SetWorldRotation` _capsulecomponent_2 (`KismetMathLibrary.MakeRotator` 0.0 (+ _returnvalue_pitch _returnvalue_y) (+ _returnvalue _returnvalue_yaw)) false false)
                    (bind _result (`/Engine/EditorBlueprintResources/StandardMacros.NegateFloat` (* _returnvalue 40.0))
                      (:`  `
                        (`SceneComponent.K2_SetRelativeRotation` (`self.Temp`) (`KismetMathLibrary.MakeRotator` 0.0 _result 90.0) false false))))))
              (:`then_1`
                (`self.AddMovementInput` (`self.GetActorForwardVector`) (/ (`KismetMathLibrary.Conv_IntToDouble` (`self.Thrust`)) 50.0))
                (set `CharacterMovementComponent.MaxFlySpeed` (`self.MaxSpeed`) (`self.CharacterMovement`)))))))
      (:`then_1`
        (if (not (`self.Autopilot`))
          ;[1 1 1] Linetrace
          (bind (_outhit _returnvalue_2) (`KismetSystemLibrary.SphereTraceSingle` (`self.K2_GetActorLocation`) (+ _worldlocation (* _worlddirection 100000.0)) 200.0 "TraceTypeQuery1"))
          (if _returnvalue_2
            (if (not (`self.TimerStarted`))
              (`self.Start Timer`)
              (elif (>= (`self.TimerSeconds`) (`self.ScannerSpeed`))
                (switch `/Game/GalaxyShooter/Blueprints/AutopilotState` (`self.AutoPilotState`)
                  (:`NewEnumerator1`
                    (`self.ClearTimer`)
                    (set `self.AutoPilotDestinationActor` (`.HitActor` (`GameplayStatics.BreakHitResult` _outhit)))
                    (set `self.Autopilot` true)
                    (bind _asbp_space_hud_2 (cast `/Game/GalaxyShooter/Game/BP_SpaceHud` (`PlayerController.GetHUD` (`GameplayStatics.GetPlayerController` 0))))
                    (bind _wbp_cursor (`/Game/GalaxyShooter/Game/BP_SpaceHud.WBP_Cursor` _asbp_space_hud_2))
                    (`/Game/GalaxyShooter/UI/Flight/WBP_Cursor.SetPercent` _wbp_cursor 0.0)
                    (`Widget.SetVisibility` _wbp_cursor "Hidden")))))
            (else
              (`self.ClearTimer`))))))))

(event `InputAxis|MouseWheel`
  (params (AxisValue :type "Float (single-precision)"))
  (bind _thrust (`self.Thrust`))
  ;[1 1 1] ThrustControllWithMouseWheel
  (if (not (`self.MineMiniGame`))
    (`|ExecutionSequence`
      (:`then_0`
        (if (> AxisValue 0.0)
          (if (< _thrust 100)
            (set `self.Thrust` (+ _thrust 10)))))
      (:`then_1`
        (if (< AxisValue 0.0)
          (if (> _thrust 0)
            (set `self.Thrust` (- _thrust 10))))))))

(event `self.ReceiveBeginPlay`
  (`EnhancedInputSubsystemInterface.AddMappingContext` (pcsubsystem `EnhancedInputLocalPlayerSubsystem` (`GameplayStatics.GetPlayerController` 0)) "/Game/GalaxyShooter/Blueprints/Inputs/SpaceshipInputs.SpaceshipInputs" 0 (struct))
  (`self.ChangeLoadUIWithStats`))

(event `self.AutoPilotDestinationSphere.OnComponentBeginOverlap`
  (params (OverlappedComponent :type "PrimitiveComponent Object Reference") (OtherActor :type "Actor Object Reference") (OtherComp :type "PrimitiveComponent Object Reference") (OtherBodyIndex :type Integer) (bFromSweep :type Boolean) (SweepResult :type "HitResult Structure (by ref)"))
  (if (and (== OtherActor (`self.AutoPilotDestinationActor`)) (`self.Autopilot`))
    (`GameplayStatics.SetGlobalTimeDilation` 1.0)
    (cast `/Game/GalaxyShooter/Blueprints/BP_Comet` OtherActor
      (:`then`
        (`self.StartMinigame`))
      (:`CastFailed`
        (cast `/Game/GalaxyShooter/Blueprints/BP_SpaceStation` OtherActor)
        (`GameplayStatics.OpenLevelBySoftObjectPtr` "/Game/GalaxyShooter/SpaceStation.SpaceStation")))))

(event `StartMinigame`
  (set `self.MineMiniGame` true)
  (`SceneComponent.K2_AddLocalRotation` (`self.Temp`) (struct :`Roll` 90.0) false false)
  (bind _asbp_space_hud (cast `/Game/GalaxyShooter/Game/BP_SpaceHud` (`PlayerController.GetHUD` (`GameplayStatics.GetPlayerController` 0))))
  (bind _wbp_minigame (`/Game/GalaxyShooter/Game/BP_SpaceHud.WBP_Minigame` _asbp_space_hud))
  (set `/Game/GalaxyShooter/UI/Flight/WBP_Minigame.currentRadius` (`/Game/GalaxyShooter/UI/Flight/WBP_Minigame.Radius` _wbp_minigame) _wbp_minigame)
  (set `/Game/GalaxyShooter/UI/Flight/WBP_Minigame.MinigameActive` true _wbp_minigame)
  (`/Game/GalaxyShooter/UI/Flight/WBP_Minigame.StartMinigame` _wbp_minigame)
  (`Widget.SetVisibility` _wbp_minigame "Visible"))

(event `EndMinigame`
  (bind _autopilotdestinationactor (`self.AutoPilotDestinationActor`))
  (set `self.MineMiniGame` false)
  (set `self.Autopilot` false)
  (set `self.Thrust` 100)
  (bind _asbp_space_hud (cast `/Game/GalaxyShooter/Game/BP_SpaceHud` (`PlayerController.GetHUD` (`GameplayStatics.GetPlayerController` 0))))
  (`Widget.SetVisibility` (`/Game/GalaxyShooter/Game/BP_SpaceHud.WBP_Cursor` _asbp_space_hud) "Visible")
  (set `self.AutoPilotState` "NewEnumerator2")
  (`NiagaraFunctionLibrary.SpawnSystemAtLocation` "/Game/GalaxyShooter/NS_DestroyedComete.NS_DestroyedComete" (`self.K2_GetActorLocation` _autopilotdestinationactor))
  (`self.K2_DestroyActor` _autopilotdestinationactor)
  (`self.ChangeLoadUIWithStats`))

(event `Start Timer`
  ;[1 1 1] Timer
  (set `self.TimerStarted` true)
  (bind _returnvalue (`KismetSystemLibrary.K2_SetTimerDelegate` (delegate `Start Timer`) 0.1 true))
  (bind _output_get (set `self.TimerSeconds` (+ (`self.TimerSeconds`) 0.1)))
  (bind _asbp_space_hud (cast `/Game/GalaxyShooter/Game/BP_SpaceHud` (`PlayerController.GetHUD` (`GameplayStatics.GetPlayerController` 0))))
  (`/Game/GalaxyShooter/UI/Flight/WBP_Cursor.SetPercent` (`/Game/GalaxyShooter/Game/BP_SpaceHud.WBP_Cursor` _asbp_space_hud) (/ _output_get (`self.ScannerSpeed`))))

(event `ClearTimer`
  ;[1 1 1] Timer
  (`KismetSystemLibrary.K2_ClearAndInvalidateTimerHandle` (stale `Start Timer` _returnvalue))
  (set `self.TimerSeconds` 0.0)
  (set `self.TimerStarted` false)
  (bind _asbp_space_hud (cast `/Game/GalaxyShooter/Game/BP_SpaceHud` (`PlayerController.GetHUD` (`GameplayStatics.GetPlayerController` 0))))
  (`/Game/GalaxyShooter/UI/Flight/WBP_Cursor.SetPercent` (`/Game/GalaxyShooter/Game/BP_SpaceHud.WBP_Cursor` _asbp_space_hud) 0.0))

(event `EnhancedInput|/Game/GalaxyShooter/Blueprints/Inputs/Interact`
  (params (ActionValue :type Boolean) (ElapsedSeconds :type "Float (double-precision)") (TriggeredSeconds :type "Float (double-precision)") (InputAction :type "InputAction Object Reference" :default "/Game/GalaxyShooter/Blueprints/Inputs/Interact.Interact"))
  (:`Completed`
    (switch `/Game/GalaxyShooter/Blueprints/AutopilotState` (`self.AutoPilotState`)
      (:`NewEnumerator2`
        (set `self.AutoPilotState` "NewEnumerator1"))
      (:`NewEnumerator1`
        (set `self.AutoPilotState` "NewEnumerator2")))))

(event `EnhancedInput|/Game/GalaxyShooter/Blueprints/Inputs/Boost`
  (params (ActionValue :type Boolean) (ElapsedSeconds :type "Float (double-precision)") (TriggeredSeconds :type "Float (double-precision)") (InputAction :type "InputAction Object Reference" :default "/Game/GalaxyShooter/Blueprints/Inputs/Boost.Boost"))
  (:`Triggered`
    (if (`self.SpeedUp`)
      (`GameplayStatics.SetGlobalTimeDilation` 1.0)
      (set `self.SpeedUp` false)
      (elif (`self.Autopilot`)
        (`GameplayStatics.SetGlobalTimeDilation` 3.0)
        (set `self.SpeedUp` true)))))

(event `self.BoxCollision.OnComponentBeginOverlap`
  (params (OverlappedComponent :type "PrimitiveComponent Object Reference") (OtherActor :type "Actor Object Reference") (OtherComp :type "PrimitiveComponent Object Reference") (OtherBodyIndex :type Integer) (bFromSweep :type Boolean) (SweepResult :type "HitResult Structure (by ref)"))
  (if (not (`self.Autopilot`))
    (bind _asbp_comet (cast `/Game/GalaxyShooter/Blueprints/BP_Comet` OtherActor))
    (`NiagaraFunctionLibrary.SpawnSystemAtLocation` "/Game/GalaxyShooter/NS_DestroyedComete.NS_DestroyedComete" (`self.K2_GetActorLocation` _asbp_comet))
    (`self.K2_DestroyActor` _asbp_comet)))

(fn `ChangeLoadUIWithStats`
  (bind _asbp_space_hud (cast `/Game/GalaxyShooter/Game/BP_SpaceHud` (`PlayerController.GetHUD` (`GameplayStatics.GetPlayerController` 0))))
  (bind _asbp_game_instance (cast `/Game/GalaxyShooter/Game/BP_GameInstance` (`GameplayStatics.GetGameInstance`)))
  (`/Game/GalaxyShooter/UI/Flight/WBP_FlightUI.ChangeLoad` (`/Game/GalaxyShooter/Game/BP_SpaceHud.WBP_FlightUI` _asbp_space_hud) (`KismetStringLibrary.Conv_IntToString` (`/Game/GalaxyShooter/Game/BP_GameInstance.ShipLoad` _asbp_game_instance)) (`KismetStringLibrary.Conv_IntToString` (`/Game/GalaxyShooter/Game/BP_GameInstance.ShipLoadMaximum` _asbp_game_instance))))

(fn `ShouldTimerStart`
  (params (ActorHit :type "Actor Object Reference"))
  (returns (Bool :type Boolean)))

(fn `UserConstructionScript`)