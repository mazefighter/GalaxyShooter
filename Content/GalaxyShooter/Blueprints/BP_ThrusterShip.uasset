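; BP_ThrusterShip is a Galaxy Shooter ship Blueprint that lets the mouse wheel adjust the strength of its PhysicsThruster component.
; Scrolling up or down raises or lowers ThrustStrength in fixed steps, with a limit check at each end of the range.
; The logic is purely input-driven, with no active Tick, BeginPlay, overlap or construction logic.
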(event `Key|MouseScrollUp`
  (params (Key :type "Key Structure"))
  (bind _physicsthruster (`self.PhysicsThruster`))
  (bind _thruststrength (`PhysicsThrusterComponent.ThrustStrength` _physicsthruster))
  (:`Pressed`
    (if (< _thruststrength 10000.0)
      (set `PhysicsThrusterComponent.ThrustStrength` (+ _thruststrength 1000.0) _physicsthruster))))

(event `Key|MouseScrollDown`
  (params (Key :type "Key Structure"))
  (bind _physicsthruster (`self.PhysicsThruster`))
  (bind _thruststrength (`PhysicsThrusterComponent.ThrustStrength` _physicsthruster))
  (:`Pressed`
    (if (> _thruststrength 1000.0)
      (set `PhysicsThrusterComponent.ThrustStrength` (- _thruststrength 1000.0) _physicsthruster))))

(fn `UserConstructionScript`)