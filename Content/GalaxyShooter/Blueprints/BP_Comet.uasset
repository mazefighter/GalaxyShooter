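; BP_Comet is a Galaxy Shooter actor that drifts and turns at random.
; A looping one-second timer calls MoveRandom, which blends the current transform toward a random nearby location and random rotation, using frame delta time as alpha.
; Tick applies the stored Destination with a swept move, so motion comes as a small step after each timer fire rather than continuous interpolation.
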(event `Move Random`
  (bind _location (.location (`self.GetTransform`)))
  (set `self.Destination` (`KismetMathLibrary.TLerp` (`KismetMathLibrary.MakeTransform` _location (.rotation (`self.GetTransform`))) (`KismetMathLibrary.MakeTransform` (+ _location (* (`KismetMathLibrary.RandomUnitVector`) 50.0)) (`KismetMathLibrary.RandomRotator` true)) (`GameplayStatics.GetWorldDeltaSeconds`))))

(event `self.ReceiveBeginPlay`
  (set `self.Destination` (`self.GetTransform`))
  (`KismetSystemLibrary.K2_SetTimerDelegate` (delegate `Move Random`) 1.0 true))

(event `self.ReceiveTick`
  (params (DeltaSeconds :type "Float (single-precision)"))
  (`self.K2_SetActorTransform` (`self.Destination`) true))

(fn `UserConstructionScript`)